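; Actor prototype for plotting data table points on a Cesium georeferenced world; none of its logic is wired to run.
; The disconnected EventGraph chain converts each row's longitude and latitude into a Niagara component position.
; It feeds "InputParam" with Speed10 normalized against the clamped range of the TSK column.
; The construction script is empty, beside an unwired variant that adds scaled mesh instances at those positions.
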(fn ConstructionScript)